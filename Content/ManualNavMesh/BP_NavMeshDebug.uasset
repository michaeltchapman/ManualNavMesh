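; Debug Blueprint for building and testing a custom manual Recast navmesh.
; It triggers the navmesh build with verbose logging and can flush debug lines.
; TestPathFinding queries a path between random WorldMap points, or TestStart and TestEnd when set, passing only direct two-point paths with matching endpoints.
; Failures print diagnostics and draw path arrows; SingleTest runs one query, while BatchTest repeats it and prints the pass count.
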(fn `BatchTest`
  (locals (SuccessCount :type Integer))
  (for _ (range (+ (`self.BatchTestCount`) 1))
    (bind _result (`self.TestPathFinding`))
    (if _result
      (`/Engine/EditorBlueprintResources/StandardMacros.IncrementInt` (`local.SuccessCount`))))
  (`KismetSystemLibrary.PrintString` (`KismetStringLibrary.Concat_StrStr` (`KismetStringLibrary.Conv_IntToString` (`local.SuccessCount`)) "/" (`KismetStringLibrary.Conv_IntToString` (`self.BatchTestCount`)) " Passed")))

(fn `BuildManualNavMesh`
  (locals (Bounds :type "Float (double-precision)"))
  (`KismetSystemLibrary.ExecuteConsoleCommand` "log LogManualNavMesh VeryVerbose" null)
  (bind _returnvalue (`ManualDetourNavMesh.GetManualRecastNavMesh` self))
  (`ManualDetourNavMesh.BuildManualNavMesh` _returnvalue))

(fn `FlushDebugLines`
  (`KismetSystemLibrary.FlushPersistentDebugLines`))

(fn `SingleTest`
  (`self.TestPathFinding`))

(fn `TestPathFinding`
  (returns (Result :type Boolean))
  (locals (NewLocalVar_0 :type "Array of Vector2D Structure") (Start :type "Vector Structure" :default (0.0 0.0 0.0)) (End :type "Vector Structure" :default (0.0 0.0 0.0)))
  (bind _worldmap (`self.WorldMap`))
  (bind _teststart (`self.TestStart`))
  (bind _testend (`self.TestEnd`))
  (bind _x (.x (`WorldMap.Max` _worldmap)))
  (bind _y (.y (`WorldMap.Max` _worldmap)))
  (bind _x_2 (.x (`WorldMap.Min` _worldmap)))
  (bind _y_2 (.y (`WorldMap.Min` _worldmap)))
  (bind _returnvalue (`ManualDetourNavMesh.GetManualRecastNavMesh` self))
  (`/Engine/EditorBlueprintResources/StandardMacros.IsValid` _returnvalue
    (:`Is Valid`
      (set `local.Start` (`KismetMathLibrary.MakeVector` (`KismetMathLibrary.RandomFloatInRange` _x_2 _x) (`KismetMathLibrary.RandomFloatInRange` _y_2 _y)))
      (set `local.End` (`KismetMathLibrary.MakeVector` (`KismetMathLibrary.RandomFloatInRange` _x_2 _x) (`KismetMathLibrary.RandomFloatInRange` _y_2 _y)))
      (if (and (`KismetSystemLibrary.IsValid` _teststart) (`KismetSystemLibrary.IsValid` _testend))
        (set `local.Start` (`self.K2_GetActorLocation` _teststart))
        (set `local.End` (`self.K2_GetActorLocation` _testend)))
      (bind _returnvalue_2 (`NavigationSystemV1.FindPathToLocationSynchronously` (`local.Start`) (`local.End`) _returnvalue null))
      (bind _pathpoints (`NavigationPath.PathPoints` _returnvalue_2))
      (bind _returnvalue_3 (`NavigationPath.IsValid` _returnvalue_2))
      (bind _returnvalue_4 (`KismetArrayLibrary.Array_Length` _pathpoints))
      (bind _returnvalue_5 (== (`local.End`) (`|GetArrayItem` _pathpoints (- _returnvalue_4 1))))
      (bind _returnvalue_6 (== _returnvalue_4 2))
      (bind _returnvalue_7 (and (== (`local.Start`) (`|GetArrayItem` _pathpoints)) _returnvalue_3 _returnvalue_5 _returnvalue_6))
      (`KismetSystemLibrary.PrintString` (`KismetStringLibrary.Concat_StrStr` " Path valid? " (`KismetStringLibrary.Conv_BoolToString` _returnvalue_7)))
      (if _returnvalue_7
        (return true)
        (else
          (`KismetSystemLibrary.PrintString` (`KismetStringLibrary.Concat_StrStr` " Length 2? " (`KismetStringLibrary.Conv_BoolToString` _returnvalue_6) " End Equal ? " (`KismetStringLibrary.Conv_BoolToString` _returnvalue_5) " Path valid? " (`KismetStringLibrary.Conv_BoolToString` _returnvalue_3)))
          (for (_array_element _array_index) _pathpoints
            (bind _returnvalue_8 (+ _array_index 1))
            (if (`KismetArrayLibrary.Array_IsValidIndex` _pathpoints _returnvalue_8)
              (`KismetSystemLibrary.DrawDebugArrow` _array_element (`|GetArrayItem` _pathpoints _returnvalue_8) 200.0 (struct :`R` 0.963542 :`B` 0.809706 :`A` 1.0) 99.0 20.0)))
          (return false))))
    (:`Is Not Valid`
      (return false))))

(fn `UserConstructionScript`)